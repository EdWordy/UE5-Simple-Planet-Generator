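; Player controller for a planet strategy layer that drives an orbit camera and handles tile selection.
; On BeginPlay it finds the planet actor and adds the strategy Enhanced Input mapping context.
; Zoom input changes the BP_OrbitCamera spring arm length, ignoring out-of-range steps, while rotate input turns the pawn in yaw and roll, not pitch.
; Left click asks the planet to select the tile under the cursor and prints the result.
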(event Input|EnhancedActionEvents|EnhancedInputActionIA_ZoomPlanet
  (params (ActionValue :type Float%20%28double-precision%29) (ElapsedSeconds :type Float%20%28double-precision%29) (TriggeredSeconds :type Float%20%28double-precision%29) (InputAction :type Input%20Action%20Object%20Reference :default "/PlanetGenerator/Input/Actions/IA_ZoomPlanet.IA_ZoomPlanet"))
  (CallFunction|ZoomCamera ActionValue))

(event Input|EnhancedActionEvents|EnhancedInputActionIA_RotatePlanet
  (params (ActionValue :type Vector%202D%20Structure) (ElapsedSeconds :type Float%20%28double-precision%29) (TriggeredSeconds :type Float%20%28double-precision%29) (InputAction :type Input%20Action%20Object%20Reference :default "/PlanetGenerator/Input/Actions/IA_RotatePlanet.IA_RotatePlanet"))
  (CallFunction|RotateCameraX (.x ActionValue))
  (CallFunction|RotateCameraY (.y ActionValue)))

(event EventBeginPlay
  (bind _returnvalue (Actor|GetActorOfClass "/Script/PlanetGenerator.PlanetActor"))
  (Variables|Default|SetPlanetActor _returnvalue)
  (Input|SetInputModeGameOnly self false)
  (Input|AddMappingContext (PlayerController|LocalPlayerSubsystems|GetEnhancedInputLocalPlayerSubsystem) "/PlanetGenerator/Input/IMC_StrategyLayer.IMC_StrategyLayer" 0 "(bIgnoreAllPressedKeysUntilRelease=True,bForceImmediately=False,bNotifyUserSettings=False)"))

(event Input|MouseEvents|LeftMouseButton
  (params (Key :type Key%20Structure :default "None"))
  (bind (_locationx _locationy) (Game|Player|GetMousePosition))
  (:Pressed
    (bind _returnvalue (Class|PlanetActor|SelectTileatScreenPosition (Variables|Default|GetPlanetActor) self (Math|Vector2D|MakeVector2D _locationx _locationy)))
    (Development|PrintString (Utilities|String|ToString(Boolean) _returnvalue))))

(fn ConstructionScript)

(fn ZoomCamera
  (params (AxisValue :type Float%20%28double-precision%29))
  (bind _asbp_orbit_camera (Utilities|Casting|CastToBP_OrbitCamera (Pawn|GetControlledPawn)))
  (if (not (or (<= (+ (Variables|/Script/Engine.SpringArmComponent|GetTargetArmLength (Variables|/PlanetGenerator/Blueprints/OrbitCam/BP_OrbitCamera.BP_OrbitCamera_C|GetSpringArm _asbp_orbit_camera)) (* AxisValue (Variables|Default|GetZoomSpeed))) 9e+03) (>= (+ (Variables|/Script/Engine.SpringArmComponent|GetTargetArmLength (Variables|/PlanetGenerator/Blueprints/OrbitCam/BP_OrbitCamera.BP_OrbitCamera_C|GetSpringArm _asbp_orbit_camera)) (* AxisValue (Variables|Default|GetZoomSpeed))) 2e+04)))
    (Variables|/Script/Engine.SpringArmComponent|SetTargetArmLength (Variables|/PlanetGenerator/Blueprints/OrbitCam/BP_OrbitCamera.BP_OrbitCamera_C|GetSpringArm _asbp_orbit_camera) (+ (Variables|/Script/Engine.SpringArmComponent|GetTargetArmLength (Variables|/PlanetGenerator/Blueprints/OrbitCam/BP_OrbitCamera.BP_OrbitCamera_C|GetSpringArm _asbp_orbit_camera)) (* AxisValue (Variables|Default|GetZoomSpeed))))))

(fn RotateCameraX
  (params (AxisX :type Float%20%28double-precision%29))
  (bind _asbp_orbit_camera (Utilities|Casting|CastToBP_OrbitCamera (Pawn|GetControlledPawn)))
  (Transformation|SetActorRotation _asbp_orbit_camera (Math|Rotator|MakeRotator (.roll (Transformation|GetActorRotation _asbp_orbit_camera)) (.pitch (Transformation|GetActorRotation _asbp_orbit_camera)) (+ (.yaw (Transformation|GetActorRotation _asbp_orbit_camera)) (* AxisX (Variables|Default|GetRotationSpeedFactor)))))
  (return))

(fn RotateCameraY
  (params (AxisY :type Float%20%28double-precision%29))
  (bind _asbp_orbit_camera (Utilities|Casting|CastToBP_OrbitCamera (Pawn|GetControlledPawn)))
  (Transformation|SetActorRotation _asbp_orbit_camera (Math|Rotator|MakeRotator (+ (.roll (Transformation|GetActorRotation _asbp_orbit_camera)) (* AxisY (Variables|Default|GetRotationSpeedFactor))) (.pitch (Transformation|GetActorRotation _asbp_orbit_camera)) (.yaw (Transformation|GetActorRotation _asbp_orbit_camera))))
  (return))